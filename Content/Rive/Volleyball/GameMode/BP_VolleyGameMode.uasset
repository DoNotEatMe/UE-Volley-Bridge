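; Volleyball game mode that sets up the match and tracks the player's successful hits and fails until a win or loss.
; BeginPlay splits AI players into teams by X position, tags and highlights a random one as the player, and has a random team's tagged server walk out, spawn and serve the ball.
; Catch events toggle the hold-Space prompt, while Updatecount updates the HUD and triggers the paused win/lose screen at either limit.
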(event Custom|PrepareToCatch
  ;[1 1 1] UI
  ;;[1 1 1] WBP Hold Space
  (bind _returnvalue (UserInterface|CreateWidget "/Game/Rive/Volleyball/UI/WBP_PlayerPrepare.WBP_PlayerPrepare_C"))
  (bind _output_get (Variables|Default|SetWBPPrepare _returnvalue))
  (UserInterface|Viewport|AddtoViewport _output_get 0)
  (Variables|/Game/Rive/Volleyball/PlayerPawn/BP_PlayerPawn.BP_PlayerPawn_C|SetCouldHitBall (Variables|Default|GetAs%20BP%20Player%20Pawn) true))

(event Custom|ClearPrepare
  ;[1 1 1] UI
  ;;[1 1 1] WBP Hold Space Remove
  (Widget|RemovefromParent (Variables|Default|GetWBPPrepare)))

(event Custom|Updatecount
  ;[1 1 1] UI
  ;;[1 1 1] Update count in UI
  (if (Variables|/Game/Rive/Volleyball/PlayerPawn/BP_PlayerPawn.BP_PlayerPawn_C|GetSpaceWasPressed (Variables|Default|GetAs%20BP%20Player%20Pawn))
    (bind _result (Math|Integer|IncrementInt (Variables|Default|GetBounceCount))
      (:%20%20
        (Default|SetBounce (Variables|Default|GetWBPCount) _result)
        (Variables|/Game/Rive/Volleyball/PlayerPawn/BP_PlayerPawn.BP_PlayerPawn_C|SetSpaceWasPressed (Variables|Default|GetAs%20BP%20Player%20Pawn) false)
        (if (== (Variables|Default|GetBounceCount) (Variables|Default|GetWinBounce))
          (CallFunction|EndGame true))))
    (else
      (bind _result_2 (Math|Integer|IncrementInt (Variables|Default|GetFailCount))
        (:%20%20
          (Default|SetFailed (Variables|Default|GetWBPCount) _result_2)
          (if (== _result_2 (Variables|Default|GetMaxFails))
            (CallFunction|ClearPrepare)
            (CallFunction|EndGame false)
            (else
              (CallFunction|ClearPrepare))))))))

(event Custom|EndGame
  (params (IsWin :type Boolean))
  (bind _returnvalue (Game|GetPlayerController 0))
  ;[1 1 1] UI
  ;;[1 1 1] End state
  (bind _returnvalue_2 (UserInterface|CreateWidget "/Game/Rive/Volleyball/UI/WBP_WinLose.WBP_WinLose_C"))
  (bind _output_get (Variables|Default|SetWBPWinLose _returnvalue_2))
  (Default|SetIsWin _output_get IsWin)
  (UserInterface|Viewport|AddtoViewport _output_get 0)
  (Input|SetInputModeUIOnly _returnvalue _output_get "DoNotLock" false)
  (Variables|/Script/Engine.PlayerController|SetbShowMouseCursor _returnvalue true)
  (Game|SetGamePaused true))

(event EventBeginPlay
  (bind _returnvalue (Game|GetPlayerController 0))
  (bind _teamb (Variables|Default|GetTeamB))
  (bind _teama (Variables|Default|GetTeamA))
  ;[1 1 1] Begin Play
  ;;[1 1 1] Recheck in case of restart
  (Input|SetInputModeGameOnly _returnvalue false)
  (Variables|/Script/Engine.PlayerController|SetbShowMouseCursor _returnvalue false)
  (bind _asbp_player_pawn (Utilities|Casting|CastToBP_PlayerPawn (Game|Player|GetPlayerPawn 0)))
  (Variables|Default|SetAs%20BP%20Player%20Pawn _asbp_player_pawn)
  ;;[1 1 1] UI for counting player points == HUD
  (bind _returnvalue_2 (UserInterface|CreateWidget "/Game/Rive/Volleyball/UI/WBP_Count.WBP_Count_C"))
  (bind _output_get (Variables|Default|SetWBPCount _returnvalue_2))
  (UserInterface|Viewport|AddtoViewport _output_get 0)
  ;;[1 1 1] Make teams based on side (simplified in case of net.X == 0.f)
  (bind _outactors (Actor|GetAllActorsOfClass "/Game/Rive/Volleyball/VolleyPlayers/BP_AIPlayer.BP_AIPlayer_C"))
  (bind _output_get_2 (Variables|Default|SetOut%20Actors _outactors))
  (for _array_element _output_get_2
    (if (> (.x (Transformation|GetActorLocation _array_element)) 0.0)
      (Variables|/Game/Rive/Volleyball/VolleyPlayers/BP_AIPlayer.BP_AIPlayer_C|SetTeam _array_element 0)
      (Utilities|Array|Add (Variables|Default|GetTeamA) _array_element)
      (else
        (Variables|/Game/Rive/Volleyball/VolleyPlayers/BP_AIPlayer.BP_AIPlayer_C|SetTeam _array_element 1)
        (Utilities|Array|Add (Variables|Default|GetTeamB) _array_element))))
  ;;[1 1 1] Choose random pawn to become player
  (Utilities|Array|Add (Variables|/Script/Engine.Actor|GetTags (Utilities|Array|Get(acopy) (Variables|Default|GetOut%20Actors) (Math|Random|RandomIntegerinRange 0 (- (Utilities|Array|Length (Variables|Default|GetOut%20Actors)) 1)))) (Variables|Default|GetPlayerTag))
  ;;[1 1 1] Player Highlight
  (bind _array_element_2 (Utilities|Array|ForEachLoopwithBreak (Variables|Default|GetOut%20Actors) :!label _label)
    (:LoopBody
      (if (Actor|ActorHasTag _array_element_2 (Variables|Default|GetPlayerTag))
        (Rendering|Material|SetMaterial (Variables|/Game/Rive/Volleyball/VolleyPlayers/BP_AIPlayer.BP_AIPlayer_C|GetCylinder _array_element_2) 0 "/Engine/EngineDebugMaterials/VertexColorViewMode_GreenOnly.VertexColorViewMode_GreenOnly")
        (goto _label Break)))
    (:Completed
      ;;[1 1 1] Spawn ball on Serve
      (if (Math|Random|RandomBool)
        (bind _array_element_3 (Utilities|Array|ForEachLoopwithBreak (Variables|Default|GetTeamA) :!label _label_2)
          (:LoopBody
            (if (Actor|ActorHasTag _array_element_3 (Variables|Default|GetServeTag))
              (bind _asbp_aiplayer (Utilities|Casting|CastToBP_AIPlayer _array_element_3))
              (bind _output_get_3 (Variables|Default|SetServeRef _asbp_aiplayer))
              (Variables|Default|SetServeStartPos (Transformation|GetActorLocation _asbp_aiplayer))
              (AI|AIMoveTo _output_get_3 (Transformation|GetActorLocation (Variables|/Game/Rive/Volleyball/VolleyPlayers/BP_AIPlayer.BP_AIPlayer_C|GetTargetPoint _asbp_aiplayer)) 0 5.0 false
                (:OnSuccess
                  (bind _returnvalue_3 (Game|SpawnActorfromClass "/Game/Rive/Volleyball/Ball/BP_Ball.BP_Ball_C" (Math|Transform|MakeTransform (Math|Vector|MakeVector (.x (Transformation|GetActorLocation (Variables|Default|GetServeRef))) (.y (Transformation|GetActorLocation (Variables|Default|GetServeRef))) (+ (.z (Transformation|GetActorLocation (Variables|Default|GetServeRef))) 1e+02)) "0, 0, 0" "1.000000,1.000000,1.000000") "Undefined" "MultiplyWithRoot" 0 0))
                  (bind _output_get_4 (Variables|Default|SetBall _returnvalue_3))
                  (Default|BallServe _output_get_4 (Variables|Default|GetServeRef) (Utilities|Array|Get(acopy) _teamb (Math|Random|RandomIntegerinRange 0 (- (Utilities|Array|Length _teamb) 1))))
                  (Development|PrintString "Team A Spawned a ball" true true "(R=1.000000,G=0.052036,B=0.000000,A=1.000000)")
                  (AI|AIMoveTo (Variables|Default|GetServeRef) (Variables|Default|GetServeStartPos) 0 5.0 false
                    (:OnSuccess
                      (goto _label_2 Break))))))))
        (else
          (bind _array_element_4 (Utilities|Array|ForEachLoopwithBreak (Variables|Default|GetTeamB) :!label _label_3)
            (:LoopBody
              (if (Actor|ActorHasTag _array_element_4 (Variables|Default|GetServeTag))
                (bind _asbp_aiplayer_2 (Utilities|Casting|CastToBP_AIPlayer _array_element_4))
                (bind _output_get_5 (Variables|Default|SetServeRef _asbp_aiplayer_2))
                (Variables|Default|SetServeStartPos (Transformation|GetActorLocation _asbp_aiplayer_2))
                (AI|AIMoveTo _output_get_5 (Transformation|GetActorLocation (Variables|/Game/Rive/Volleyball/VolleyPlayers/BP_AIPlayer.BP_AIPlayer_C|GetTargetPoint _asbp_aiplayer_2)) 0 5.0 false
                  (:OnSuccess
                    (bind _returnvalue_4 (Game|SpawnActorfromClass "/Game/Rive/Volleyball/Ball/BP_Ball.BP_Ball_C" (Math|Transform|MakeTransform (Math|Vector|MakeVector (.x (Transformation|GetActorLocation (Variables|Default|GetServeRef))) (.y (Transformation|GetActorLocation (Variables|Default|GetServeRef))) (+ (.z (Transformation|GetActorLocation (Variables|Default|GetServeRef))) 1e+02)) "0, 0, 0" "1.000000,1.000000,1.000000") "Undefined" "MultiplyWithRoot" 0 0))
                    (bind _output_get_6 (Variables|Default|SetBall _returnvalue_4))
                    (Default|BallServe _output_get_6 (Variables|Default|GetServeRef) (Utilities|Array|Get(acopy) _teama (Math|Random|RandomIntegerinRange 0 (- (Utilities|Array|Length _teama) 1))))
                    (Development|PrintString "Team B Spawned a ball" true true "(R=1.000000,G=0.052036,B=0.000000,A=1.000000)")
                    (Utilities|FlowControl|Delay 0.2)
                    (AI|AIMoveTo (Variables|Default|GetServeRef) (Variables|Default|GetServeStartPos) 0 5.0 false
                      (:OnSuccess
                        (goto _label_3 Break)))))))))))))

(fn ConstructionScript)