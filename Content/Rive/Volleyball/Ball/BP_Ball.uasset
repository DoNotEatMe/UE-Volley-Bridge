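; Volleyball actor that launches itself between players of two teams in a continuous rally.
; BallServe computes a ballistic impulse peaking above the net and landing on the receiver, sending AI receivers to a randomly offset spot or opening the game mode's catch window for the player.
; A new player hit resets physics, counts player touches, returns the receiver to its start and serves to a random opponent, ignoring repeat hits.
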(event OnComponentHit(Sphere)
  (params (HitComponent :type Primitive%20Component%20Object%20Reference) (OtherActor :type Actor%20Object%20Reference) (OtherComp :type Primitive%20Component%20Object%20Reference) (NormalImpulse :type Vector :default "0, 0, 0") (Hit :type Hit%20Result%20Structure%20%28by%20ref%29))
  (bind _as_volley_game_mode (Variables|Default|GetAs%20Volley%20Game%20Mode))
  (bind _as_volley_game_mode_2 (Variables|Default|GetAs%20Volley%20Game%20Mode))
  (bind _sphere (Variables|Default|GetSphere))
  (bind _teama (Variables|/Game/Rive/Volleyball/GameMode/BP_VolleyGameMode.BP_VolleyGameMode_C|GetTeamA _as_volley_game_mode))
  (bind _teamb (Variables|/Game/Rive/Volleyball/GameMode/BP_VolleyGameMode.BP_VolleyGameMode_C|GetTeamB _as_volley_game_mode_2))
  ;[1 1 1] Check last hitted actor to avoid hit stack
  (bind _asbp_aiplayer (Utilities|Casting|CastToBP_AIPlayer OtherActor))
  (bind _output_get (Variables|Default|SetAs%20Character _asbp_aiplayer))
  (if (not (== _output_get (Variables|Default|GetLastHitActor)))
    ;[1 1 1] Add match point if player hit the ball
    (if (Actor|ActorHasTag (Variables|Default|GetAs%20Character) "Player")
      (Default|Updatecount (Variables|Default|GetAs%20Volley%20Game%20Mode)))
    ;[1 1 1] ZVelocity
    (Physics|SetPhysicsLinearVelocity (Variables|Default|GetSphere) "0, 0, 0" false "None")
    (Class|PrimitiveComponent|SetPhysicsAngularVelocityinDegrees (Variables|Default|GetSphere) "0, 0, 0" false "None")
    (Physics|SetSimulatePhysics _sphere false)
    (Physics|SetSimulatePhysics _sphere true)
    (Default|MovetoPick (Variables|Default|GetAs%20AI%20receiver) (Variables|Default|GetAI%20Start%20Pos))
    (Variables|Default|SetSender (Variables|Default|GetReceiver))
    (bind _asbp_aiplayer_2 (Utilities|Casting|CastToBP_AIPlayer (Variables|Default|GetSender)))
    (bind _output_get_2 (Variables|Default|SetAs%20BP%20AIPlayer _asbp_aiplayer_2))
    (if (== (Variables|/Game/Rive/Volleyball/VolleyPlayers/BP_AIPlayer.BP_AIPlayer_C|GetTeam _output_get_2) 0)
      (bind _asbp_aiplayer_3 (Utilities|Casting|CastToBP_AIPlayer (Utilities|Array|Get(acopy) _teamb (Math|Random|RandomIntegerinRange 0 (- (Utilities|Array|Length _teamb) 1)))))
      (CallFunction|BallServe (Variables|/Game/Rive/Volleyball/GameMode/BP_VolleyGameMode.BP_VolleyGameMode_C|GetBall (Variables|Default|GetAs%20Volley%20Game%20Mode)) (Variables|Default|GetAs%20BP%20AIPlayer) _asbp_aiplayer_3)
      (Variables|Default|SetLastHitActor (Variables|Default|GetAs%20BP%20AIPlayer))
      (else
        (bind _asbp_aiplayer_4 (Utilities|Casting|CastToBP_AIPlayer (Utilities|Array|Get(acopy) _teama (Math|Random|RandomIntegerinRange 0 (- (Utilities|Array|Length _teama) 1)))))
        (CallFunction|BallServe (Variables|/Game/Rive/Volleyball/GameMode/BP_VolleyGameMode.BP_VolleyGameMode_C|GetBall (Variables|Default|GetAs%20Volley%20Game%20Mode)) (Variables|Default|GetAs%20BP%20AIPlayer) _asbp_aiplayer_4)
        (Variables|Default|SetLastHitActor (Variables|Default|GetAs%20BP%20AIPlayer))))))

(event Custom|BallServe
  (params (Sender :type Character%20Object%20Reference) (Receiver :type Character%20Object%20Reference))
  (bind _sphere (Variables|Default|GetSphere))
  (Variables|Default|SetSender Sender)
  (bind _output_get (Variables|Default|SetReceiver Receiver))
  (bind _asbp_aiplayer (Utilities|Casting|CastToBP_AIPlayer _output_get))
  (Variables|Default|SetAs%20AI%20receiver _asbp_aiplayer)
  (Variables|Default|SetAI%20Start%20Pos (Transformation|GetActorLocation (Variables|Default|GetAs%20AI%20receiver)))
  (if (Actor|ActorHasTag _output_get "Player")
    (Variables|Default|SetTarget%20Pos (Transformation|GetActorLocation _output_get))
    ;[1 1 1] Tap window
    (Default|PreparetoCatch (Variables|Default|GetAs%20Volley%20Game%20Mode))
    (else
      (bind _output_get_2 (Variables|Default|SetTarget%20Pos (+ (Transformation|GetActorLocation _output_get) (Math|Vector|MakeVector (Math|Random|RandomFloatinRange 0.0 1e+02) (Math|Random|RandomFloatinRange 0.0 1e+02) 0.0))))
      (Default|MovetoPick (Variables|Default|GetAs%20AI%20receiver) _output_get_2)))
  (Variables|Default|SetCurrentPos (Transformation|GetWorldLocation (Variables|Default|GetSphere)))
  ;[1 1 1] Ball Physics logic
  ;;[1 1 1] Height needed to avoid net
  (bind _output_get_3 (Variables|Default|SetPeakHeight (+ (Variables|Default|GetNetHeight) (Math|Random|RandomFloatinRange 1.5e+02 2e+02))))
  (bind _output_get_4 (Variables|Default|SetHeightDifferenceAscent%20 (- _output_get_3 (.z (Variables|Default|GetCurrentPos)))))
  (bind _output_get_5 (Variables|Default|SetHeightDifferenceDescent%20 (- _output_get_3 (.z (Variables|Default|GetTarget%20Pos)))))
  (if (and (> _output_get_4 0.0) (> _output_get_5 0.0))
    (bind _output_get_6 (Variables|Default|SetTimeToPeak (Math|Float|Sqrt (/ (* (Variables|Default|GetHeightDifferenceAscent%20) 2.0) (Variables|Default|GetGravity)))))
    (bind _output_get_7 (Variables|Default|SetTimeToDescend%20 (Math|Float|Sqrt (/ (* (Variables|Default|GetHeightDifferenceDescent%20) 2.0) (Variables|Default|GetGravity)))))
    (Variables|Default|SetTotalTimeOfFlight%20 (+ _output_get_6 _output_get_7))
    (bind _output_get_8 (Variables|Default|SetDistanceX%20 (- (.x (Variables|Default|GetTarget%20Pos)) (.x (Variables|Default|GetCurrentPos)))))
    (bind _output_get_9 (Variables|Default|SetDistanceY (- (.y (Variables|Default|GetTarget%20Pos)) (.y (Variables|Default|GetCurrentPos)))))
    (Physics|AddImpulse _sphere (* (Math|Vector|MakeVector (/ _output_get_8 (Variables|Default|GetTotalTimeOfFlight%20)) (/ _output_get_9 (Variables|Default|GetTotalTimeOfFlight%20)) (* (Variables|Default|GetGravity) (Variables|Default|GetTimeToPeak))) (Physics|GetMass _sphere)) "None" false)
    (else
      (Development|PrintString "HeightDifference is bad"))))

(event Custom|VisualizeVelocity
  (bind _sphere (Variables|Default|GetSphere))
  (bind _returnvalue (Transformation|GetWorldLocation _sphere))
  (bind _returnvalue_2 (Physics|GetPhysicsLinearVelocity (Variables|Default|GetSphere) "None"))
  (Rendering|Debug|DrawDebugLine _returnvalue (* (+ _returnvalue_2 _returnvalue) 1.0) "(R=0.000000,G=1.000000,B=0.114498,A=1.000000)" -1.0 0.0))

(event EventTick
  (params (DeltaSeconds :type Float%20%28single-precision%29)))

(event EventBeginPlay
  (bind _asbp_volley_game_mode (Utilities|Casting|CastToBP_VolleyGameMode (Game|GetGameMode))
    (:then
      (Variables|Default|SetAs%20Volley%20Game%20Mode _asbp_volley_game_mode))
    (:CastFailed
      (Development|PrintString "BP_Ball Get GameMode in Begin Play Failed"))))

(fn ConstructionScript)