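; BP_PlayerPawn is the player pawn for the volleyball game, handling the input to hit the ball.
; On BeginPlay it resets CouldHitBall, adds the IMC_main Enhanced Input mapping context and caches BP_VolleyGameMode.
; When IA_Space triggers while CouldHitBall is true, it sets SpaceWasPressed and calls ClearPrepare on the game mode.
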(event Input|EnhancedActionEvents|EnhancedInputActionIA_Space
  (params (ActionValue :type Boolean) (ElapsedSeconds :type Float%20%28double-precision%29) (TriggeredSeconds :type Float%20%28double-precision%29) (InputAction :type Input%20Action%20Object%20Reference :default "/Game/Rive/Volleyball/IA/IA_Space.IA_Space"))
  (:Triggered
    (if (Variables|Default|GetCouldHitBall)
      (Variables|Default|SetSpaceWasPressed true)
      (Default|ClearPrepare (Variables|Default|GetAs%20Volley%20Game%20Mode)))))

(event EventBeginPlay
  (bind _returnvalue (Game|GetPlayerController 0))
  (bind _returnvalue_2 (PlayerController|LocalPlayerSubsystems|GetEnhancedInputLocalPlayerSubsystem _returnvalue))
  (Variables|Default|SetCouldHitBall false)
  (Utilities|IsValid _returnvalue_2
    (:Is%20Valid
      (Input|AddMappingContext _returnvalue_2 "/Game/Rive/Volleyball/IA/IMC_main.IMC_main" 0 "(bIgnoreAllPressedKeysUntilRelease=True,bForceImmediately=False,bNotifyUserSettings=False)")
      (bind _asvolley_game_mode (Utilities|Casting|CastToBP_VolleyGameMode (Game|GetGameMode)))
      (Variables|Default|SetAs%20Volley%20Game%20Mode _asvolley_game_mode))
    (:Is%20Not%20Valid
      (Development|PrintString "Enhanced Input Local Player Subsystem is not valid"))))

(event Collision|EventActorBeginOverlap
  (params (OtherActor :type Actor%20Object%20Reference)))

(event EventTick
  (params (DeltaSeconds :type Float%20%28single-precision%29)))

(fn ConstructionScript)