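; Physics rope bridge actor that sways as if in wind.
; The construction script lays a row of plank meshes along local Y from the bridge length, links neighbours with physics constraints and pins both end planks.
; A looping timer, its interval randomised once at BeginPlay, applies random mass-scaled impulses to roughly a third of the inner planks.
; A start-to-end point variant of the build is present but unconnected.
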(event EventBeginPlay
  (Utilities|Time|SetTimerbyFunctionName 0 "Impulse" (Math|Random|RandomFloatinRange 0.3 1.0) true))

(event EventTick
  (params (DeltaSeconds :type Float%20%28single-precision%29)))

(fn ConstructionScript
  (bind _planks (Variables|Default|GetPlanks))
  (bind _planks_2 (Variables|Default|GetPlanks))
  (if (not (<= (Variables|Default|GetBridgeLenght) 0.0))
    ;[1 1 1] fixed lenght
    (bind _output_get (Variables|Default|SetPlanksCount (/ (Variables|Default|GetBridgeLenght) 0.7)))
    ;;[1 1 1] Generate Planks
    (for _index (range 0 (- _output_get 1))
      (bind _returnvalue (AddComponent|AddStaticMeshComponent false (Math|Transform|MakeTransform (Math|Vector|MakeVector 0.0 (Math|Conversions|ToFloat(Integer) (* _index 70)) 0.0) "0, 0, 0" "1.000000,1.000000,1.000000")))
      (Utilities|Array|Add (Variables|Default|GetPlanks) _returnvalue))
    ;;[1 1 1] Generate Constraints
    (for _index_2 (range 0 (- (Variables|Default|GetPlanksCount) 2))
      (bind _returnvalue_2 (AddComponent|AddPhysicsConstraintComponent false (Math|Transform|MakeTransform (Math|Vector|MakeVector 0.0 (+ (.y (Variables|/Script/Engine.SceneComponent|GetRelativeLocation (Utilities|Array|Get(acopy) (Variables|Default|GetPlanks) _index_2))) 35.0) 0.0) "0.000000,0.000000,90.000000" "1.000000,1.000000,1.000000")))
      (Class|PhysicsConstraintComponent|SetConstrainedComponents _returnvalue_2 (Utilities|Array|Get(acopy) _planks _index_2) "None" (Utilities|Array|Get(acopy) _planks (+ _index_2 1)) "None"))
    (Physics|SetSimulatePhysics (Utilities|Array|Get(acopy) _planks_2) false)
    (Physics|SetSimulatePhysics (Utilities|Array|Get(acopy) _planks_2 (Utilities|Array|LastIndex _planks_2)) false)))

(fn Impulse
  (bind _returnvalue (Math|Random|RandomFloatinRange -1e+03 1e+03))
  (bind _planks (Variables|Default|GetPlanks))
  (bind _returnvalue_2 (Utilities|Array|Length _planks))
  (bind _returnvalue_3 (- _returnvalue_2 2))
  (bind _returnvalue_4 (Math|Random|RandomIntegerinRange 1 _returnvalue_3))
  (bind _output (Utilities|Array|Get(acopy) _planks _returnvalue_4))
  (for _index (range 0 (/ _returnvalue_3 3))
    (bind _output_get (Variables|Default|SetWind%20Impulse (Math|Vector|MakeVector _returnvalue _returnvalue (Math|Random|RandomFloatinRange -1e+02 1e+02))))
    (Physics|AddImpulse _output (* (Physics|GetMass _output) _output_get) "None" false)))